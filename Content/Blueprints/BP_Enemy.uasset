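; BP_Enemy is an enemy actor with a health bar widget that reacts to being hit by projectiles.
; BeginPlay caches the BP_Enemy_Health widget from the EnemyHealth widget component, and Tick sets its progress bar from Health as a fraction of 100.
; A hit from a Projectile turns on physics simulation on the Mesh, but nothing in this graph changes Health.
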(event EventBeginPlay
  (bind _asbp_enemy_health (Utilities|Casting|CastToBP_Enemy_Health (UserInterface|GetUserWidgetObject (Variables|Default|GetEnemy%20Health))))
  (Variables|Default|SetEnemy%20Health%20UI%20REF _asbp_enemy_health))

(event Collision|EventActorBeginOverlap
  (params (OtherActor :type Actor%20Object%20Reference)))

(event EventTick
  (params (DeltaSeconds :type Float%20%28single-precision%29))
  (Progress|SetPercent (Variables|/Game/Blueprints/BP_Enemy_Health.BP_Enemy_Health_C|GetHealth_Progress_Bar (Variables|Default|GetEnemy%20Health%20UI%20REF)) (/ (Variables|Default|GetHealth) 1e+02)))

(event Collision|EventHit
  (params (MyComp :type Primitive%20Component%20Object%20Reference) (Other :type Actor%20Object%20Reference) (OtherComp :type Primitive%20Component%20Object%20Reference) (bSelfMoved :type Boolean) (HitLocation :type Vector :default "0, 0, 0") (HitNormal :type Vector :default "0, 0, 0") (NormalImpulse :type Vector :default "0, 0, 0") (Hit :type Hit%20Result%20Structure%20%28by%20ref%29))
  (Utilities|Casting|CastToProjectile Other)
  (Physics|SetSimulatePhysics (Variables|Character|GetMesh) true))

(fn ConstructionScript)